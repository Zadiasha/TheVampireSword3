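; BPC_Health_Enemy is a health component for enemies that tracks current health against a maximum.
; It refills health to the maximum on BeginPlay through Recovery, which is also a callable function.
; AddHealth and Damage adjust the value, clamped at the maximum and at zero, while GetHealth and IsDead expose the state.
; When Damage brings health to zero, a DoOnce gate guards the OnDead dispatcher call.
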(event EventBeginPlay
  (CallFunction|Recovery))

(event EventTick
  (params (DeltaSeconds :type Float%20%28single-precision%29)))

(fn GetHealth
  (return (Variables|Default|GetHealth)))

(fn IsDead
  (return (<= (Variables|Default|GetHealth) 0.0)))

(fn AddHealth
  (params (AddHealth :type Float%20%28single-precision%29))
  (Variables|Default|SetHealth (Math|Float|Min(Float) (+ AddHealth (Variables|Default|GetHealth)) (Variables|Default|GetMax%20Health)))
  (return))

(fn Damage
  (params (Damage :type Float%20%28single-precision%29))
  (bind _output_get (Variables|Default|SetHealth (Math|Float|Max(Float) (- (Variables|Default|GetHealth) Damage) 0.0)))
  (if (<= _output_get 0.0)
    (Utilities|FlowControl|DoOnce false
      (:Completed
        (Default|CallOnDead)))))

(fn Recovery
  (Variables|Default|SetHealth (Variables|Default|GetMax%20Health))
  (return))