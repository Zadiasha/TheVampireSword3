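; Serf enemy character Blueprint with melee great sword attacks, health and a floating HP bar that turns toward the player's follow camera.
; Attack stops movement and plays one of two random montages behind a DoOnce that attackended resets while restoring speed.
; A toggled attack capsule damages overlapped actors through a second DoOnce, reset when the capsule is disabled.
; Lethal damage notifies the AnimBP, disables collision and destroys the actor after a delay.
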(event OnComponentBeginOverlap(attackcapsule)
  (params (OverlappedComponent :type Primitive%20Component%20Object%20Reference) (OtherActor :type Actor%20Object%20Reference) (OtherComp :type Primitive%20Component%20Object%20Reference) (OtherBodyIndex :type Integer) (bFromSweep :type Boolean) (SweepResult :type Hit%20Result%20Structure%20%28by%20ref%29))
  (if (!= OtherActor self)
    (Utilities|FlowControl|DoOnce false
      (:Completed
        (Game|Damage|ApplyDamage OtherActor (Math|Random|RandomFloatinRange (Variables|Default|Getbase%20damage) (Variables|Default|Getbase%20damage)) 0 0)))))

(event Custom|Attack
  (if (not (Variables|Default|GetIs%20Dead?))
    (Utilities|FlowControl|DoOnce false
      (:Completed
        (Variables|/Script/Engine.CharacterMovementComponent|SetMaxWalkSpeed (Variables|Character|GetCharacterMovement) 0.0)
        (if (Math|Random|RandomBoolwithWeight 0.5)
          (Animation|PlayAnimMontage "/Game/EnemyCarSettings/EnemyChar2/Animations/Great_Sword_Attack_Montage.Great_Sword_Attack_Montage" 0.7 "None")
          (else
            (Animation|PlayAnimMontage "/Game/EnemyCarSettings/EnemyChar2/Animations/Great_Sword_Slash_Montage.Great_Sword_Slash_Montage" 0.7 "None")))))))

(event Custom|attack%20ended
  (Variables|/Script/Engine.CharacterMovementComponent|SetMaxWalkSpeed (Variables|Character|GetCharacterMovement) (Variables|Default|GetStart%20Max%20Speed))
  (Utilities|FlowControl|DoOnce false) ; enters at Reset
)

(event Custom|Enable%20attack%20capsule
  (Collision|SetCollisionEnabled (Variables|Default|Getattackcapsule) "QueryOnly"))

(event Custom|disable%20attack%20capsule
  (Collision|SetCollisionEnabled (Variables|Default|Getattackcapsule) "NoCollision")
  (CallFunction|RefrashAttackCapsule))

(event Custom|Refrash%20attack%20capsule
  (Utilities|FlowControl|DoOnce false) ; enters at Reset
)

(event Custom|Death
  (Variables|Default|SetIs%20Dead? true)
  (Default|DeathonAnimBP (.AsSerf%20BP (Utilities|Casting|CastToSerfBP (Components|SkeletalMesh|GetAnimInstance (Variables|Character|GetMesh)))))
  (Animation|StopAnimMontage "/Game/EnemyCarSettings/EnemyChar2/Animations/Great_Sword_Attack_Montage.Great_Sword_Attack_Montage")
  (Animation|StopAnimMontage "/Game/EnemyCarSettings/EnemyChar2/Animations/Great_Sword_Slash_Montage.Great_Sword_Slash_Montage")
  (Collision|SetCollisionEnabled (Variables|Collision|GetCapsuleComponent) "NoCollision")
  (Collision|SetCollisionEnabled (Variables|Default|Getattackcapsule) "NoCollision")
  (Utilities|FlowControl|Delay 15.0)
  (Actor|DestroyActor))

(event EventBeginPlay
  (Variables|Default|SetHpBarSerfWidgetRef (.AsHp%20Bar%20Serf%20Widget (Utilities|Casting|CastToHp_Bar_Serf_Widget (UserInterface|GetUserWidgetObject (Variables|Default|GetHpBar%20Serf)))))
  (Variables|Default|SetStart%20Max%20Speed (Variables|/Script/Engine.CharacterMovementComponent|GetMaxWalkSpeed (Variables|Character|GetCharacterMovement))))

(event Game|Damage|EventAnyDamage
  (params (Damage :type Float%20%28single-precision%29) (DamageType :type Damage%20Type%20Object%20Reference) (InstigatedBy :type Controller%20Object%20Reference) (DamageCauser :type Actor%20Object%20Reference))
  (if (not (Variables|Default|GetIs%20Dead?))
    (bind _output_get (Variables|Default|SetCurrentHP (Math|Float|SelectFloat 0.0 (- (Variables|Default|GetCurrentHP) Damage) (>= Damage (Variables|Default|GetCurrentHP)))))
    (Utilities|FlowControl|Sequence
      (:then_1
        (if (<= _output_get 0.0)
          (CallFunction|Death))))))

(event EventTick
  (params (DeltaSeconds :type Float%20%28single-precision%29))
  (Utilities|FlowControl|Sequence
    (:then_0
      ;[0.369 1 0.2027] Widget
      (Progress|SetPercent (Variables|/Game/EnemyCarSettings/EnemyChar2/Hp_Bar_Serf_Widget.Hp_Bar_Serf_Widget_C|GetHPBar (Variables|Default|GetHpBarSerfWidgetRef)) (Math|Float|NormalizetoRange (Variables|Default|GetCurrentHP) 0.0 (Variables|Default|GetMaxHP))))
    (:then_1
      ;;[1 1 1] Отображение Виджета
      (Transformation|SetWorldRotation (Variables|Default|GetHpBar%20Serf) (Math|Rotator|FindLookatRotation (Transformation|GetWorldLocation (Variables|Default|GetHpBar%20Serf)) (Transformation|GetWorldLocation (Variables|/Game/ThirdPersonBP/Blueprints/ThirdPersonCharacter.ThirdPersonCharacter_C|GetFollowCamera (.AsThird%20Person%20Character (Utilities|Casting|CastToThirdPersonCharacter (Game|GetPlayerCharacter 0)))))) false false))))

(fn ConstructionScript)

(fn GetDamage
  (return (Math|Random|RandomFloatinRange (Variables|Default|Getbase%20damage) (Variables|Default|Getbase%20damage))))